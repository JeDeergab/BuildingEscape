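; An openable door actor that swings open and shut when its OpenDoor member fires open and close events.
; BeginPlay caches the initial rotation, which a timeline combines with an animated yaw angle to rotate the whole actor.
; Opening plays the timeline and closing reverses it, while a timeline event track times the door lock sound at the actor's location.
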(event `self.ReceiveBeginPlay`
  ;[1 1 1] Sets the rotation for the OpenDoor only to be use globally
  (set `self.Initial Rotation` (`self.K2_GetActorRotation`)))

(event `self.OpenDoor.OnOpenDoor`
  ;[1 1 1] Creates Rotating Animation for OpenDoor
  (bind (_direction _openangle) (`Timeline|Timeline_0` :!label _label)
    (:`Update`
      (`self.K2_SetActorRotation` (`KismetMathLibrary.ComposeRotators` (`KismetMathLibrary.MakeRotator` 0.0 0.0 _openangle) (`self.Initial Rotation`))))
    (:`Sound Timing`
      ;[1 1 1] Adding Sounds
      (`GameplayStatics.PlaySoundAtLocation` "/Game/Audio/door-lock.door-lock" (`self.K2_GetActorLocation`)))))

(event `self.OpenDoor.OnCloseDoor`
  ;[1 1 1] Creates Rotating Animation for OpenDoor
  (goto _label :!via `Reverse`))

(fn `UserConstructionScript`)